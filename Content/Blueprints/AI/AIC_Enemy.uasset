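; AI controller for enemies that runs the BT_Enemy behavior tree on the BB_Enemy blackboard.
; On BeginPlay it sets the player's BP_Captain as attack target as a temporary aggro system, storing it in the blackboard and a variable.
; On possess it binds to the BP_ActionChar pawn's stun state event and mirrors stun changes into a blackboard bool.
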(event Custom|OnStunStateChanged
  (params (IsStunned :type Boolean))
  (AI|Components|Blackboard|SetValueasBool (Variables|Default|GetBlackboard) (Variables|Default|GetIsStunnedKey) IsStunned))

(event EventBeginPlay
  (Class|AIController|UseBlackboard "/Game/Blueprints/AI/BB_Enemy.BB_Enemy")
  (AI|RunBehaviorTree "/Game/Blueprints/AI/BT_Enemy.BT_Enemy")
  ;[1 1 1] Temporary aggro system
  (bind _asbp_captain (Utilities|Casting|CastToBP_Captain (Game|Player|GetPlayerPawn 0)))
  (CallFunction|SetAttackTarget _asbp_captain))

(event EventTick
  (params (DeltaSeconds :type Float%20%28single-precision%29)))

(event EventPossess
  (params (PossessedPawn :type Pawn%20Object%20Reference))
  (bind _asbp_action_char (Utilities|Casting|CastToBP_ActionChar PossessedPawn))
  (EventDispatchers|BindEventtoStunStateChanged _asbp_action_char (delegate Custom|OnStunStateChanged)))

(fn ConstructionScript)

(fn SetAttackTarget
  (params (AttackTarget :type BP%20Captain%20Object%20Reference))
  (AI|Components|Blackboard|SetValueasObject (AI|GetBlackboard 0) (Variables|Default|GetAttackTargetKey) AttackTarget)
  (Variables|Default|SetAttackTarget AttackTarget))